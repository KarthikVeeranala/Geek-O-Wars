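; Player character with camera-relative movement, jumping and a two-slot weapon inventory.
; Pickups respawn as primary or secondary weapons attached to holster sockets, and equip and switch inputs move them to and from the GunHold socket while setting WeaponState.
; When armed, aiming toggles controller-yaw rotation.
; Held fire loops through a Gate and retriggerable delay, playing montage and sound, decrementing ammo and running debug-drawn camera line traces whose hits are unused.
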(event `InputAxis|MoveForBack`
  (params (AxisValue :type "Float (single-precision)"))
  (bind (_returnvalue_roll _returnvalue_pitch _returnvalue_yaw) (`KismetMathLibrary.BreakRotator` (`self.GetControlRotation`)))
  (`self.AddMovementInput` (`KismetMathLibrary.GetForwardVector` (`KismetMathLibrary.MakeRotator` 0.0 0.0 _returnvalue_yaw)) AxisValue))

(event `InputAxis|MoveRightLeft`
  (params (AxisValue :type "Float (single-precision)"))
  (bind (_returnvalue_roll _returnvalue_pitch _returnvalue_yaw) (`KismetMathLibrary.BreakRotator` (`self.GetControlRotation`)))
  (`self.AddMovementInput` (`KismetMathLibrary.GetRightVector` (`KismetMathLibrary.MakeRotator` 0.0 0.0 _returnvalue_yaw)) AxisValue))

(event `InputAction|Jump`
  (params (Key :type "Key Structure"))
  (:`Pressed`
    (`self.Jump`)))

(event `InputAxis|MouseYaw`
  (params (AxisValue :type "Float (single-precision)"))
  (`self.AddControllerYawInput` AxisValue))

(event `InputAxis|MousePitch`
  (params (AxisValue :type "Float (single-precision)"))
  (`self.AddControllerPitchInput` AxisValue))

(event `Pickupitem`
  (params (NewItem :type "/Game/GameBluePrint/WeaponBP/BPM_Weapon Object Reference"))
  (bind ((`WeaponClass_5_AE3B57B14AD85D307D8F469B882D2E8C` _weaponclass) (`UnequipSocket_13_6258EB90427429CAD6D292A10DD7575F` _unequipsocket)) (break `/Game/GameBluePrint/WeaponBP/WeaponInfo` (`/Game/GameBluePrint/WeaponBP/BPM_Weapon.WeaponInfo` (`self.Weapon cache`))))
  (bind ((`WeaponClass_5_AE3B57B14AD85D307D8F469B882D2E8C` _weaponclass_2) (`UnequipSocket_13_6258EB90427429CAD6D292A10DD7575F` _unequipsocket_2)) (break `/Game/GameBluePrint/WeaponBP/WeaponInfo` (`/Game/GameBluePrint/WeaponBP/BPM_Weapon.WeaponInfo` (`self.Weapon cache`))))
  (set `self.Weapon cache` NewItem)
  (`self.PrimaryBP`
    (:`then`
      (`self.SecondaryBP`
        (:`then`)
        (:`else`
          (bind _returnvalue (`|SpawnActorFromClass` _weaponclass (`SceneComponent.GetSocketTransform` (`self.Mesh`) _unequipsocket "RTS_World") "Undefined" "OverrideRootScale" null null))
          (bind _output_get (set `self.SecondaryBP` _returnvalue))
          (`/Game/GameBluePrint/WeaponBP/BPM_Weapon.ClearALl` _output_get)
          (`self.K2_AttachToComponent` _output_get (`self.Mesh`) (`.UnequipSocket_13_6258EB90427429CAD6D292A10DD7575F` (break `/Game/GameBluePrint/WeaponBP/WeaponInfo` (`/Game/GameBluePrint/WeaponBP/BPM_Weapon.WeaponInfo` _output_get))) "SnapToTarget" "SnapToTarget" "SnapToTarget" true)
          (`self.K2_DestroyActor` (`self.Weapon cache`)))))
    (:`else`
      (bind _returnvalue_2 (`|SpawnActorFromClass` _weaponclass_2 (`SceneComponent.GetSocketTransform` (`self.Mesh`) _unequipsocket_2 "RTS_World") "Undefined" "OverrideRootScale" null null))
      (bind _output_get_2 (set `self.PrimaryBP` _returnvalue_2))
      (set `self.CurrentWeaponBP` _output_get_2)
      (`/Game/GameBluePrint/WeaponBP/BPM_Weapon.ClearALl` _output_get_2)
      (`self.K2_AttachToComponent` _output_get_2 (`self.Mesh`) (`.UnequipSocket_13_6258EB90427429CAD6D292A10DD7575F` (break `/Game/GameBluePrint/WeaponBP/WeaponInfo` (`/Game/GameBluePrint/WeaponBP/BPM_Weapon.WeaponInfo` _output_get_2))) "SnapToTarget" "SnapToTarget" "SnapToTarget" true)
      (`self.K2_DestroyActor` (`self.Weapon cache`)))))

(event `EquipSwitch`
  (bind _secondarybp (`self.SecondaryBP`))
  (bind _primarybp (`self.PrimaryBP`))
  (if (or (`KismetSystemLibrary.IsValid` (`self.PrimaryBP`)) (`KismetSystemLibrary.IsValid` (`self.SecondaryBP`))) :!label _label
    (if (== (`self.PrimaryBP`) (`self.CurrentWeaponBP`))
      (if (`|EnumEquality` (`self.WeaponState`) "NewEnumerator1")
        (set `self.WeaponState` "NewEnumerator0" :!label _label_2)
        (`self.K2_AttachToComponent` _primarybp (`self.Mesh`) (`.UnequipSocket_13_6258EB90427429CAD6D292A10DD7575F` (break `/Game/GameBluePrint/WeaponBP/WeaponInfo` (`/Game/GameBluePrint/WeaponBP/BPM_Weapon.WeaponInfo` _primarybp))) "SnapToTarget" "SnapToTarget" "SnapToTarget" true)
        (else
          (bind _output_get (set `self.CurrentWeaponBP` (`self.PrimaryBP`) :!label _label_3))
          (set `self.WeaponState` "NewEnumerator1")
          (`self.K2_AttachToComponent` _output_get (`self.Mesh`) "GunHold" "SnapToTarget" "SnapToTarget" "SnapToTarget" true)))
      (else
        (if (`KismetSystemLibrary.IsValid` (`self.SecondaryBP`)) :!label _label_4
          (if (== (`self.SecondaryBP`) (`self.CurrentWeaponBP`))
            (if (`|EnumEquality` (`self.WeaponState`) "NewEnumerator2")
              (set `self.WeaponState` "NewEnumerator0" :!label _label_5)
              (`self.K2_AttachToComponent` _secondarybp (`self.Mesh`) (`.UnequipSocket_13_6258EB90427429CAD6D292A10DD7575F` (break `/Game/GameBluePrint/WeaponBP/WeaponInfo` (`/Game/GameBluePrint/WeaponBP/BPM_Weapon.WeaponInfo` _secondarybp))) "SnapToTarget" "SnapToTarget" "SnapToTarget" true)
              (else
                (bind _output_get_2 (set `self.CurrentWeaponBP` (`self.SecondaryBP`) :!label _label_6))
                (set `self.WeaponState` "NewEnumerator2")
                (`self.K2_AttachToComponent` _output_get_2 (`self.Mesh`) "GunHold" "SnapToTarget" "SnapToTarget" "SnapToTarget" true)))))))
    (else
      (goto _label_4))))

(event `InputAction|Equip`
  (params (Key :type "Key Structure"))
  (:`Pressed`
    (goto _label)))

(event `InputAction|SwitchWeapon`
  (params (Key :type "Key Structure"))
  (:`Pressed`
    (if (`KismetSystemLibrary.IsValid` (`self.PrimaryBP`))
      (if (`|EnumEquality` (`self.WeaponState`) "NewEnumerator1")
        (`|ExecutionSequence`
          (:`then_0`
            (goto _label_2))
          (:`then_1`
            (goto _label_6)))
        (else
          _)))
    (if (`KismetSystemLibrary.IsValid` (`self.SecondaryBP`))
      (if (`|EnumEquality` (`self.WeaponState`) "NewEnumerator2")
        (`|ExecutionSequence`
          (:`then_0`
            (goto _label_5))
          (:`then_1`
            (goto _label_3)))
        (else
          (`self.EquipSwitch`))))))

(event `InputAction|Aiming`
  (params (Key :type "Key Structure"))
  (bind _charactermovement (`self.CharacterMovement`))
  (:`Pressed`
    (if (`|EnumInequality` (`self.WeaponState`) "NewEnumerator0")
      (`/Engine/EditorBlueprintResources/StandardMacros.FlipFlop`
        (:`A`
          (set `self.IsAiming` true)
          (set `self.bUseControllerRotationYaw` true)
          (set `CharacterMovementComponent.bOrientRotationToMovement` false _charactermovement))
        (:`B`
          (set `self.IsAiming` false)
          (set `self.bUseControllerRotationYaw` false)
          (set `CharacterMovementComponent.bOrientRotationToMovement` true _charactermovement))))))

(event `InputAction|Fire`
  (params (Key :type "Key Structure"))
  (bind _camera (`self.Camera`))
  (bind _returnvalue (`SceneComponent.K2_GetComponentLocation` _camera))
  (bind ((`Range_18_A167713847F621C2BCC3D2A37E73B16C` _range) (`FireSound_43_5C8CAAC3438523B3A1658682CB86A088` _firesound)) (break `/Game/GameBluePrint/WeaponBP/WeaponInfo` (`/Game/GameBluePrint/WeaponBP/BPM_Weapon.WeaponInfo` (`self.CurrentWeaponBP`))))
  (:`Pressed`
    (if (`|EnumInequality` (`self.WeaponState`) "NewEnumerator0")
      (`|ExecutionSequence`
        (:`then_0`
          (goto _label_7 :!via `Open`))
        (:`then_1`
          (`/Engine/EditorBlueprintResources/StandardMacros.Gate` true :!label _label_7
            (:`Exit`
              (`|ExecutionSequence`
                (:`then_0`
                  (`KismetSystemLibrary.RetriggerableDelay` (`.FireRate_35_7E298A104D73AEBA3EA9F2AB18902E49` (break `/Game/GameBluePrint/WeaponBP/WeaponInfo` (`/Game/GameBluePrint/WeaponBP/BPM_Weapon.WeaponInfo` (`self.CurrentWeaponBP`)))))
                  (goto _label_7))
                (:`then_1`
                  (if (== (`.CurrentAmmo_24_79F1CFC84DF155C2AF3E85A20057BA97` (break `/Game/GameBluePrint/WeaponBP/WeaponInfo` (`/Game/GameBluePrint/WeaponBP/BPM_Weapon.WeaponInfo` (`self.CurrentWeaponBP`)))) 0)
                    (`self.StopFire`)
                    (else
                      (`self.PlayAnimMontage` "/Game/AnimStarterPack/Fire_Rifle_Ironsights_Montage.Fire_Rifle_Ironsights_Montage")
                      (`GameplayStatics.PlaySound2D` _firesound 1.0 1.0 0.0 null null)
                      (`KismetSystemLibrary.LineTraceSingle` :`Start` _returnvalue :`End` (+ _returnvalue (* (`SceneComponent.GetForwardVector` _camera) _range)) :`TraceChannel` "TraceTypeQuery1" :`DrawDebugType` "ForDuration" :`DrawTime` 2.0)
                      (`/Engine/EditorBlueprintResources/StandardMacros.DecrementInt` (`.CurrentAmmo_24_79F1CFC84DF155C2AF3E85A20057BA97` (break `/Game/GameBluePrint/WeaponBP/WeaponInfo` (`/Game/GameBluePrint/WeaponBP/BPM_Weapon.WeaponInfo` (`self.CurrentWeaponBP`)))))))))))))))
  (:`Released`
    (goto _label_7 :!via `Close`)))

(event `StopFire`
  (goto _label_7 :!via `Close`))

(fn `Equipment`
  (params (`Weapon Ref` :type "/Game/GameBluePrint/WeaponBP/BPM_Weapon Object Reference"))
  (set `self.WeaponState` "NewEnumerator0")
  (`self.K2_AttachToComponent` `Weapon Ref` (`self.Mesh`) (`.EquipSocket_11_B59782774FFF0E5509396A99F6EDD149` (break `/Game/GameBluePrint/WeaponBP/WeaponInfo` (`/Game/GameBluePrint/WeaponBP/BPM_Weapon.WeaponInfo` `Weapon Ref`))) "KeepRelative" "KeepRelative" "KeepRelative" true))

(fn `Unequipment`
  (params (`Weapon Ref` :type "/Game/GameBluePrint/WeaponBP/BPM_Weapon Object Reference"))
  (set `self.WeaponState` "NewEnumerator0")
  (`self.K2_AttachToComponent` `Weapon Ref` (`self.Mesh`) (`.UnequipSocket_13_6258EB90427429CAD6D292A10DD7575F` (break `/Game/GameBluePrint/WeaponBP/WeaponInfo` (`/Game/GameBluePrint/WeaponBP/BPM_Weapon.WeaponInfo` `Weapon Ref`))) "KeepRelative" "KeepRelative" "KeepRelative" true))

(fn `UserConstructionScript`)